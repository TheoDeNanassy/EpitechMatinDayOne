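; BP_Cone is a level piece that acts as either a safe zone or a falling hazard for the player, chosen by IsConeSafe.
; Safe instances swap their mesh to a plains floor on BeginPlay.
; Box overlaps pass the flag to BP_MyPlayer's SetSafeZone and clear it on exit.
; When the player enters an unsafe instance, the mesh starts simulating physics after a delay, and the actor later destroys itself.
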(event `self.ReceiveBeginPlay`
  (if (`self.IsConeSafe?`)
    (`StaticMeshComponent.SetStaticMesh` (`self.Cone`) "/Game/InfinityBladeGrassLands/Environments/Plains/Env_Plains_Ruins/StaticMesh/SM_Plains_Floor_01.SM_Plains_Floor_01")))

(event `self.Box.OnComponentBeginOverlap`
  (params (OverlappedComponent :type "PrimitiveComponent Object Reference") (OtherActor :type "Actor Object Reference") (OtherComp :type "PrimitiveComponent Object Reference") (OtherBodyIndex :type Integer) (bFromSweep :type Boolean) (SweepResult :type "HitResult Structure (by ref)"))
  (bind _asbp_my_player (cast `/Game/Blueprints/BP_MyPlayer` OtherActor))
  (`/Game/Blueprints/BP_MyPlayer.SetSafeZone` _asbp_my_player (`self.IsConeSafe?`))
  (if (not (`self.IsConeSafe?`))
    (`KismetSystemLibrary.Delay` 3.0)
    (`PrimitiveComponent.SetSimulatePhysics` (`self.Cone`) true)
    (`KismetSystemLibrary.Delay` 10.0)
    (`self.K2_DestroyActor`)))

(event `self.Box.OnComponentEndOverlap`
  (params (OverlappedComponent :type "PrimitiveComponent Object Reference") (OtherActor :type "Actor Object Reference") (OtherComp :type "PrimitiveComponent Object Reference") (OtherBodyIndex :type Integer))
  (bind _asbp_my_player (cast `/Game/Blueprints/BP_MyPlayer` OtherActor))
  (`/Game/Blueprints/BP_MyPlayer.SetSafeZone` _asbp_my_player false))

(fn `UserConstructionScript`)