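; BP_Cube is a cube actor that is either safe or periodically disappears, depending on its IsSafeCube flag.
; On BeginPlay, a safe cube takes the EmisiveCubeSafe material and stays solid.
; Any other cube starts a looping HideCube timer, with its interval randomized once at startup.
; Each tick of that timer toggles both visibility and collision, so the cube alternates between hidden, passable and visible, solid.
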(event `self.ReceiveBeginPlay`
  (if (`self.IsSafeCube?`)
    (`PrimitiveComponent.SetMaterial` (`self.Cube`) 0 "/Game/Materials/EmisiveCubeSafe.EmisiveCubeSafe")
    (else
      (`KismetSystemLibrary.K2_SetTimer` null "HideCube" (`KismetMathLibrary.RandomFloatInRange` 3.0 8.0) true))))

(fn `HideCube`
  (bind _cube (`self.Cube`))
  (bind _cube_2 (`self.Cube`))
  (if (not (`SceneComponent.bHiddenInGame` (`self.Cube`)))
    (`SceneComponent.SetHiddenInGame` _cube_2 true false)
    (`PrimitiveComponent.SetCollisionEnabled` _cube_2 "NoCollision")
    (else
      (`SceneComponent.SetHiddenInGame` _cube false false)
      (`PrimitiveComponent.SetCollisionEnabled` _cube "QueryAndPhysics"))))

(fn `UserConstructionScript`)