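; Turret Blueprint that turns toward the player and fires projectiles while the player is inside its detection sphere and outside a safe zone.
; Sphere overlap, gated by a cooldown flag, fires immediately and starts looping aim and fire timers sharing one random delay, with fire slightly after aim.
; Leaving clears those timers and ticks down MyCD each second to control the flag; MyCD is never reset here.
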(event `self.Sphere.OnComponentBeginOverlap`
  (params (OverlappedComponent :type "PrimitiveComponent Object Reference") (OtherActor :type "Actor Object Reference") (OtherComp :type "PrimitiveComponent Object Reference") (OtherBodyIndex :type Integer) (bFromSweep :type Boolean) (SweepResult :type "HitResult Structure (by ref)"))
  (bind _asbp_my_player (cast `/Game/Blueprints/BP_MyPlayer` OtherActor))
  (set `self.MyPlayer` _asbp_my_player)
  (if (and (`self.IsCDGood`) (not (`/Game/Blueprints/BP_MyPlayer.SafeZone?` _asbp_my_player)))
    (`self.MoveToPlayer`)
    (`self.F_SpawnProjectile`)
    (bind _output_get (set `self.MyRandomAttackDelay` (`KismetMathLibrary.RandomFloatInRange` 5.0 10.0)))
    (`KismetSystemLibrary.K2_SetTimer` null "MoveToPlayer" _output_get true)
    (`KismetSystemLibrary.K2_SetTimer` null "F_SpawnProjectile" (+ _output_get 0.25) true)))

(event `self.Sphere.OnComponentEndOverlap`
  (params (OverlappedComponent :type "PrimitiveComponent Object Reference") (OtherActor :type "Actor Object Reference") (OtherComp :type "PrimitiveComponent Object Reference") (OtherBodyIndex :type Integer))
  (cast `/Game/Blueprints/BP_MyPlayer` OtherActor)
  (`KismetSystemLibrary.K2_SetTimer` null "DecreaseCD" 1.0 true)
  (`KismetSystemLibrary.K2_ClearTimer` null "F_SpawnProjectile")
  (`KismetSystemLibrary.K2_ClearTimer` null "MoveToPlayer"))

(fn `DecreaseCD`
  (bind _output_get (set `self.MyCD` (- (`self.MyCD`) 1.0)))
  (if (<= _output_get 0.0)
    (set `self.MyCD` 0.0)
    (set `self.IsCDGood` true)
    (`KismetSystemLibrary.K2_ClearTimer` null "DecreaseCD")
    (else
      (set `self.IsCDGood` false))))

(fn `F_SpawnProjectile`
  (if (not (`/Game/Blueprints/BP_MyPlayer.SafeZone?` (`self.MyPlayer`)))
    (`|SpawnActorFromClass` "/Game/Blueprints/BP_Projectile.BP_Projectile_C" (`KismetMathLibrary.MakeTransform` (`SceneComponent.K2_GetComponentLocation` (`self.SpawnProjectile`)) (`self.PlayerRot`)) "Undefined" "OverrideRootScale" null null)
    (`GameplayStatics.PlaySound2D` "/Game/StarterContent/Audio/Explosion01.Explosion01" 1.0 1.0 0.0 null null)))

(fn `MoveToPlayer`
  (if (not (`/Game/Blueprints/BP_MyPlayer.SafeZone?` (`self.MyPlayer`)))
    (bind _output_get (set `self.PlayerRot` (`KismetMathLibrary.FindLookAtRotation` (`self.K2_GetActorLocation`) (`self.K2_GetActorLocation` (`GameplayStatics.GetPlayerCharacter` 0)))))
    (`self.K2_SetActorRotation` _output_get)))

(fn `UserConstructionScript`)